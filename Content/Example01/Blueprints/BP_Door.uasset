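; BP_Door is a door that toggles open and closed whenever its attached button is pressed.
; On BeginPlay it binds to the button's press event, which flips the open state and plays or reverses a timeline.
; The timeline lerps the door's relative rotation through a quarter turn, then broadcasts DoorStateUpdated with the current state when finished.
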(event `self.ReceiveBeginPlay`
  (add `/Game/Example01/Blueprints/BP_Button.ButtonPressed` (`self.AttachedButton`) (delegate `OpenCloseDoor`)))

(event `OpenCloseDoor`
  (bind _output_get (set `self.bDoorIsOpen` (not (`self.bDoorIsOpen`))))
  (if _output_get
    (bind (_direction _0_1lerp) (`Timeline|Timeline_Door` :!label _label)
      (:`Update`
        (`SceneComponent.K2_SetRelativeRotation` (`self.Door`) (`KismetMathLibrary.RLerp` (struct :`Yaw` 180.0) (struct :`Yaw` 90.0) _0_1lerp true) false false))
      (:`Finished`
        (`self.DoorStateUpdated` (`self.bDoorIsOpen`))))
    (else
      (goto _label :!via `Reverse`))))

(fn `UserConstructionScript`)