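; BP_Button is an interactable button that fires a press event and animates its top sinking when used.
; Its Box overlap events tell the player pawn, via interface messages, when it enters or leaves the interact zone.
; The Interact event calls the ButtonPressed dispatcher, then plays a timeline that lerps the ButtonTop component's relative Z downward along a curve.
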(event `self.Box.OnComponentBeginOverlap`
  (params (OverlappedComponent :type "PrimitiveComponent Object Reference") (OtherActor :type "Actor Object Reference") (OtherComp :type "PrimitiveComponent Object Reference") (OtherBodyIndex :type Integer) (bFromSweep :type Boolean) (SweepResult :type "HitResult Structure (by ref)"))
  (bind _returnvalue (`GameplayStatics.GetPlayerPawn` 0))
  (if (== OtherActor _returnvalue)
    (message `/Game/Shared/Blueprints/BPI_Interact.EnterInteractZone` _returnvalue self)))

(event `/Game/Shared/Blueprints/BPI_Interact.Interact`
  (params (CallingActor :type "Actor Object Reference"))
  (`|ExecutionSequence`
    (:`then_0`
      (`self.ButtonPressed`))
    (:`then_1`
      (bind (_direction _lerpcurve) (`Timeline|ButtonPress_Animation` :!via `PlayFromStart`)
        (:`Update`
          (`SceneComponent.K2_SetRelativeLocation` (`self.ButtonTop`) (`KismetMathLibrary.MakeVector` 0.0 0.0 (`KismetMathLibrary.Lerp` 0.0 -4.0 _lerpcurve)) false false))))))

(event `self.Box.OnComponentEndOverlap`
  (params (OverlappedComponent :type "PrimitiveComponent Object Reference") (OtherActor :type "Actor Object Reference") (OtherComp :type "PrimitiveComponent Object Reference") (OtherBodyIndex :type Integer))
  (bind _returnvalue (`GameplayStatics.GetPlayerPawn` 0))
  (if (== OtherActor _returnvalue)
    (message `/Game/Shared/Blueprints/BPI_Interact.EndedInteractZone` _returnvalue self)))

(fn `UserConstructionScript`)